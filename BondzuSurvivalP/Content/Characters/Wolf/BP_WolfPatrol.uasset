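; Wolf AI character that patrols a linked chain of BP_PatrolPoint actors and chases the player on sight.
; The patrol graph moves to GoalActor, then advances to that point's NextPoint after a short delay and repeats.
; PawnSensing triggers a move toward player zero, and patrol resumes after a delay only if that move fails.
; An idle-animation pause before patrolling is present but unconnected.
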(event OnSeePawn(PawnSensing)
  (params (Pawn :type Pawn%20Object%20Reference))
  (AI|AIMoveTo self "0, 0, 0" (Game|GetPlayerCharacter 0) 5.0 true
    (:OnFail
      (Utilities|FlowControl|Delay 5.0)
      (Utilities|PatrollingBehaivoir))))

(event EventBeginPlay
  (Utilities|PatrollingBehaivoir))

(fn ConstructionScript)