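; BP_Wolf is a wolf AI character that roams at random and chases the player once pawn sensing sees a pawn.
; FreeRoam loops moves to random reachable points with pauses, playing a breathing idle when a move fails.
; A sighting sets flags and starts AIMoveTo toward the player; nothing here clears them.
; Tick's look-at rotation targets the wolf's own location rather than the player's, and the animation Blueprint hookup is disconnected.
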(event OnSeePawn(PawnSensing)
  (params (Pawn :type Pawn%20Object%20Reference))
  (Variables|Default|SetcanLookAtPlayer true)
  (Development|PrintString "Can see the player")
  (Variables|Default|SetisSeeingPlayer true)
  (CallFunction|FollowPlayer))

(event Custom|FollowPlayer
  (if (Variables|Default|GetisSeeingPlayer)
    (AI|AIMoveTo self "420.000000,1193.000000,50.000000" (Game|GetPlayerCharacter 0) 5.0 false)))

(event Custom|FreeRoam
  (AI|AIMoveTo self (.RandomLocation (AI|Navigation|GetRandomReachablePointinRadius (Transformation|GetActorLocation) 1e+03 0 0)) 0 5.0 false
    (:OnSuccess
      (Utilities|FlowControl|Delay 4.0)
      (CallFunction|FreeRoam))
    (:OnFail
      (Components|Animation|SetAnimation (Variables|Character|GetMesh) "/Game/Characters/Wolf/Breathing_Idle.Breathing_Idle")
      (Utilities|FlowControl|Delay 4.0)
      (CallFunction|FreeRoam))))

(event EventTick
  (params (DeltaSeconds :type Float%20%28single-precision%29))
  (if (Variables|Default|GetcanLookAtPlayer)
    (Transformation|SetActorRotation (Math|Interpolation|RInterpTo (Transformation|GetActorRotation) (Math|Rotator|FindLookatRotation (Transformation|GetActorLocation) (Transformation|GetActorLocation)) DeltaSeconds 5.0))))

(event EventBeginPlay
  (CallFunction|FreeRoam))

(fn ConstructionScript)