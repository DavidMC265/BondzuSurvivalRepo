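; Enemy character that wanders the level and chases the player once its PawnSensing component sees a pawn.
; FreeRoam loops AI MoveTo to random reachable nearby points, pausing after each successful move.
; Sighting sets IsSeeingPlayer, which is never cleared here, and FollowPlayer moves toward player 0.
; BeginPlay starts roaming and caches EnmyAnim_BP, but the CanRunToPlayer update and another FreeRoam restart are unwired.
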(event OnSeePawn(PawnSensing)
  (params (Pawn :type Pawn%20Object%20Reference))
  (Development|PrintString "Can see the player")
  (Variables|Default|SetisSeeingPlayer true)
  (CallFunction|FollowPlayer))

(event Custom|FollowPlayer
  (if (Variables|Default|GetisSeeingPlayer)
    (AI|AIMoveTo self "420.000000,1193.000000,50.000000" (Game|GetPlayerCharacter 0) 5.0 false)))

(event Custom|FreeRoam
  (AI|AIMoveTo self (.RandomLocation (AI|Navigation|GetRandomReachablePointinRadius (Transformation|GetActorLocation) 1e+03 0 0)) 0 5.0 false
    (:OnSuccess
      (Utilities|FlowControl|Delay 4.0)
      (CallFunction|FreeRoam))))

(event EventBeginPlay
  (CallFunction|FreeRoam)
  (bind _asenmy_anim_bp (Utilities|Casting|CastToEnmyAnim_BP (Components|SkeletalMesh|GetAnimInstance (Variables|Character|GetMesh))))
  (Variables|Default|SetEnemy%20Animation%20blueprint _asenmy_anim_bp))

(fn ConstructionScript)